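; BP_ItemBulletBox is an ammo pickup that adds bullets to one of the player's weapons.
; When its static mesh begins overlapping a BP_MainGamePlayer, a DoOnce lets the grant fire a single time.
; It picks a random index within the player's WeaponBulletCount array and increases that count using the box's IncreaseBulletCount array.
; The graph does not destroy or hide the box afterward.
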(event OnComponentBeginOverlap(StaticMesh)
  (params (OverlappedComponent :type Primitive%20Component%20Object%20Reference) (OtherActor :type Actor%20Object%20Reference) (OtherComp :type Primitive%20Component%20Object%20Reference) (OtherBodyIndex :type Integer) (bFromSweep :type Boolean) (SweepResult :type Hit%20Result%20Structure%20%28by%20ref%29))
  (bind _asbp_main_game_player (Utilities|Casting|CastToBP_MainGamePlayer OtherActor))
  (Utilities|FlowControl|DoOnce false
    (:Completed
      (Utilities|Array|SetArrayElem (Variables|/Game/Blueprint/Gamemode/MainGame/BP_MainGamePlayer.BP_MainGamePlayer_C|GetWeaponBulletCount _asbp_main_game_player) (Math|Random|RandomIntegerinRange 0 (Utilities|Array|LastIndex (Variables|/Game/Blueprint/Gamemode/MainGame/BP_MainGamePlayer.BP_MainGamePlayer_C|GetWeaponBulletCount _asbp_main_game_player))) (+ (Utilities|Array|Get(acopy) (Variables|/Game/Blueprint/Gamemode/MainGame/BP_MainGamePlayer.BP_MainGamePlayer_C|GetWeaponBulletCount _asbp_main_game_player) (Math|Random|RandomIntegerinRange 0 (Utilities|Array|LastIndex (Variables|/Game/Blueprint/Gamemode/MainGame/BP_MainGamePlayer.BP_MainGamePlayer_C|GetWeaponBulletCount _asbp_main_game_player)))) (Utilities|Array|Get(acopy) (Variables|Default|GetIncreaseBulletCount) (Math|Random|RandomIntegerinRange 0 (Utilities|Array|LastIndex (Variables|/Game/Blueprint/Gamemode/MainGame/BP_MainGamePlayer.BP_MainGamePlayer_C|GetWeaponBulletCount _asbp_main_game_player)))))))))

(fn ConstructionScript
  (|CallParentFunction))