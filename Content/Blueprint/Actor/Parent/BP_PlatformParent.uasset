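; Parent platform tile for an endlessly generated course, randomly building floors, an obstacle and stars as child actors on BeginPlay.
; Floors fill three two-slot columns with one guaranteed, and the respawn point follows a filled column.
; Falling players respawn there and lose HP, while overlapping GenerateTile asks BP_MainGamemode for the next tile once.
; Leaving Box destroys the tile after a delay, unless Tick has seen the player dead.
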(event OnComponentHit(PlayerDropCollision)
  (params (HitComponent :type Primitive%20Component%20Object%20Reference) (OtherActor :type Actor%20Object%20Reference) (OtherComp :type Primitive%20Component%20Object%20Reference) (NormalImpulse :type Vector :default "0, 0, 0") (Hit :type Hit%20Result%20Structure%20%28by%20ref%29))
  ;[1 1 1] 플레이어가 떨어질 경우 리스폰
  (bind _asbp_main_game_player (Utilities|Casting|CastToBP_MainGamePlayer OtherActor))
  (Transformation|SetActorTransform _asbp_main_game_player (Transformation|GetWorldTransform (Variables|Default|GetRespawnPlayerPos)))
  ;[1 1 1] 리스폰시 체력 감소
  (bind _asbp_main_game_player_2 (Utilities|Casting|CastToBP_MainGamePlayer (Game|GetPlayerCharacter 0)))
  (Variables|/Game/Blueprint/Gamemode/MainGame/BP_MainGamePlayer.BP_MainGamePlayer_C|SetCurrentHP _asbp_main_game_player_2 (- (Variables|/Game/Blueprint/Gamemode/MainGame/BP_MainGamePlayer.BP_MainGamePlayer_C|GetCurrentHP _asbp_main_game_player_2) 1.0)))

(event OnComponentBeginOverlap(GenerateTile)
  (params (OverlappedComponent :type Primitive%20Component%20Object%20Reference) (OtherActor :type Actor%20Object%20Reference) (OtherComp :type Primitive%20Component%20Object%20Reference) (OtherBodyIndex :type Integer) (bFromSweep :type Boolean) (SweepResult :type Hit%20Result%20Structure%20%28by%20ref%29))
  ;[1 1 1] 다음 타일 생성
  (Utilities|Casting|CastToBP_MainGamePlayer OtherActor)
  (bind _asbp_main_gamemode (Utilities|Casting|CastToBP_MainGamemode (Game|GetGameMode)))
  (Utilities|FlowControl|DoOnce false
    (:Completed
      (Default|AddTile _asbp_main_gamemode))))

(event OnComponentEndOverlap(Box)
  (params (OverlappedComponent :type Primitive%20Component%20Object%20Reference) (OtherActor :type Actor%20Object%20Reference) (OtherComp :type Primitive%20Component%20Object%20Reference) (OtherBodyIndex :type Integer))
  ;[1 1 1] 액터 파괴
  (if (Variables|Default|GetIsDelete)
    (Utilities|FlowControl|Delay 1e+01)
    (Actor|DestroyActor)))

(event EventBeginPlay
  ;[1 1 1] 바닥, 장애물 및 코인 생성
  (CallFunction|MakeFloor)
  (CallFunction|SetRespawnPos)
  (CallFunction|MakeObstacle)
  (CallFunction|MakeCoin))

(event EventTick
  (params (DeltaSeconds :type Float%20%28single-precision%29))
  (bind _asbp_main_game_player (Utilities|Casting|CastToBP_MainGamePlayer (Game|GetPlayerCharacter 0)))
  (if (Variables|/Game/Blueprint/Gamemode/MainGame/BP_MainGamePlayer.BP_MainGamePlayer_C|GetIsDeath _asbp_main_game_player)
    (Variables|Default|SetIsDelete false)
    (else
      (Variables|Default|SetIsDelete true))))

(fn ConstructionScript
  (CallFunction|SetFloorNum)
  (CallFunction|SetFloorPosition)
  (CallFunction|SetObstaclePosition)
  (CallFunction|SetCoinPosition))

(fn MakeObstacle
  (if (> (LocalVariables|GetObstaclePercent) (Math|Random|RandomFloatinRange 0.0 1.0))
    (bind _returnvalue (AddComponent|AddChildActorComponent false (Utilities|Array|Get(acopy) (Variables|DefaultLocation|GetObstaclePos) (Math|Random|RandomIntegerinRange 0 1))))
    (ChildActorComponent|SetChildActorClass _returnvalue "/Game/Blueprint/Actor/BP_ObstacleNormal.BP_ObstacleNormal_C")))

(fn MakeCoin
  (for _index (range 0 (Utilities|Array|LastIndex (Variables|DefaultLocation|GetCoinPos)))
    (if (> (LocalVariables|GetCoinPercent) (Math|Random|RandomFloatinRange 0.0 1.0))
      (bind _returnvalue (AddComponent|AddChildActorComponent false (Utilities|Array|Get(acopy) (Variables|DefaultLocation|GetCoinPos) _index)))
      (ChildActorComponent|SetChildActorClass _returnvalue "/Game/Blueprint/Actor/BP_Star.BP_Star_C"))))

(fn SetObstaclePosition
  (Variables|DefaultLocation|SetObstaclePos (Utilities|Array|MakeArray (Transformation|GetRelativeTransform (Variables|Default|GetObstacleSector1Back)) (Transformation|GetRelativeTransform (Variables|Default|GetObstacleSector1Front)))))

(fn SetCoinPosition
  (Variables|DefaultLocation|SetCoinPos (Utilities|Array|MakeArray (Transformation|GetRelativeTransform (Variables|Default|GetCoinSector1MidProntLeft)) (Transformation|GetRelativeTransform (Variables|Default|GetCoinSector1MidProntRight)) (Transformation|GetRelativeTransform (Variables|Default|GetCoinSector1MidBackLeft)) (Transformation|GetRelativeTransform (Variables|Default|GetCoinSector1MidBackRight)) (Transformation|GetRelativeTransform (Variables|Default|GetCoinSector1BackLeft)) (Transformation|GetRelativeTransform (Variables|Default|GetCoinSector1BackRight)))))

(fn MakeFloor
  (CallFunction|MakeMinimumFloor (Math|Random|RandomIntegerinRange 0 2))
  (CallFunction|AddFloor 0 2)
  (CallFunction|SpawnFloor))

(fn SetFloorPosition
  (Variables|DefaultLocation|SetFloorPos (Utilities|Array|MakeArray (Transformation|GetRelativeTransform (Variables|Default|GetFloorPos00)) (Transformation|GetRelativeTransform (Variables|Default|GetFloorPos01)) (Transformation|GetRelativeTransform (Variables|Default|GetFloorPos02)) (Transformation|GetRelativeTransform (Variables|Default|GetFloorPos03)) (Transformation|GetRelativeTransform (Variables|Default|GetFloorPos04)) (Transformation|GetRelativeTransform (Variables|Default|GetFloorPos05)))))

(fn SetFloorNum
  (Variables|DefaultLocation|SetFloorNum (Utilities|Array|MakeArray 0 1 2 3 4 5)))

(fn MakeMinimumFloor
  (params (Offset :type Integer))
  (for _index (range 0 1)
    (Utilities|Array|SetArrayElem (Variables|Default|GetCanGenerateFloor) (+ (* _index 3) Offset) true)))

(fn AddFloor
  (params (MinOffset :type Integer) (MaxOffset :type Integer))
  (for _index (range MinOffset MaxOffset)
    (if (not (Utilities|Array|Get(acopy) (Variables|Default|GetCanGenerateFloor) _index))
      (LocalVariables|SetTempBool (Math|Random|RandomBool))
      (for _index_2 (range 0 1)
        (Utilities|Array|SetArrayElem (Variables|Default|GetCanGenerateFloor) (+ (* _index_2 3) _index) (LocalVariables|GetTempBool))))))

(fn SpawnFloor
  (bind _cangeneratefloor (Variables|Default|GetCanGenerateFloor))
  (bind _generatefloor (LocalVariables|GetGenerateFloor))
  (for _index (range 0 (Utilities|Array|LastIndex _cangeneratefloor))
    (if (Utilities|Array|Get(acopy) _cangeneratefloor _index)
      (bind _returnvalue (Utilities|Array|Add _generatefloor (Utilities|Array|Get(acopy) (Variables|DefaultLocation|GetFloorPos) _index)))
      (bind _returnvalue_2 (AddComponent|AddChildActorComponent false (Utilities|Array|Get(acopy) _generatefloor _returnvalue)))
      (ChildActorComponent|SetChildActorClass _returnvalue_2 "/Game/Blueprint/Actor/BP_Floor2.BP_Floor2_C"))))

(fn SetRespawnPos
  (for _index (range 0 2)
    (if (Utilities|Array|Get(acopy) (Variables|Default|GetCanGenerateFloor) _index)
      (Transformation|SetRelativeTransform (Variables|Default|GetRespawnPlayerPos) (Utilities|Array|Get(acopy) (Variables|DefaultLocation|GetRespawnPos) _index) false false))))