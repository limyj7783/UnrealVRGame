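; BP_SmallDartPlatformParent is a parent actor for small dart targets that award score when shot.
; Its construction script rolls a small random AddScore and shows it on the TextRender.
; When a BP_BulletParent overlaps the static mesh, it adds AddScore multiplied by the bullet's ScoreRate to the BP_MainGamePlayer's CurrentScore, then destroys itself.
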(event OnComponentBeginOverlap(StaticMesh)
  (params (OverlappedComponent :type Primitive%20Component%20Object%20Reference) (OtherActor :type Actor%20Object%20Reference) (OtherComp :type Primitive%20Component%20Object%20Reference) (OtherBodyIndex :type Integer) (bFromSweep :type Boolean) (SweepResult :type Hit%20Result%20Structure%20%28by%20ref%29))
  (bind _asbp_bullet_parent (Utilities|Casting|CastToBP_BulletParent OtherActor))
  (bind _asbp_main_game_player (Utilities|Casting|CastToBP_MainGamePlayer (Game|GetPlayerCharacter 0)))
  (Variables|/Game/Blueprint/Gamemode/MainGame/BP_MainGamePlayer.BP_MainGamePlayer_C|SetCurrentScore _asbp_main_game_player (+ (Variables|/Game/Blueprint/Gamemode/MainGame/BP_MainGamePlayer.BP_MainGamePlayer_C|GetCurrentScore _asbp_main_game_player) (* (Variables|Default|GetAddScore) (Variables|/Game/Blueprint/Actor/Parent/BP_BulletParent.BP_BulletParent_C|GetScoreRate _asbp_bullet_parent))))
  (Actor|DestroyActor))

(event EventBeginPlay)

(event Collision|EventActorBeginOverlap
  (params (OtherActor :type Actor%20Object%20Reference)))

(event EventTick
  (params (DeltaSeconds :type Float%20%28single-precision%29)))

(fn ConstructionScript
  (bind _output_get (Variables|Default|SetAddScore (Math|Random|RandomIntegerinRange 1 15)))
  (Rendering|Components|TextRender|SetText (Variables|Default|GetTextRender) (Utilities|Text|ToText(Integer) _output_get)))