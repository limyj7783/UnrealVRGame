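; BP_LobbyPlatform is a self-recycling lobby platform segment built from BP_Floor2 child actors.
; Construction runs SetFloorNum and SetFloorPosition, and BeginPlay spawns a floor child actor at each FloorPos transform.
; When a BP_LoobyPlayer enters the GenerateTile trigger, it asks BP_Lobbymode once to add the next start tile.
; The platform destroys itself after a short delay once the player leaves the trigger.
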(event OnComponentBeginOverlap(GenerateTile)
  (params (OverlappedComponent :type Primitive%20Component%20Object%20Reference) (OtherActor :type Actor%20Object%20Reference) (OtherComp :type Primitive%20Component%20Object%20Reference) (OtherBodyIndex :type Integer) (bFromSweep :type Boolean) (SweepResult :type Hit%20Result%20Structure%20%28by%20ref%29))
  ;[1 1 1] 다음 타일 생성
  (Utilities|Casting|CastToBP_LoobyPlayer OtherActor)
  (bind _asbp_lobbymode (Utilities|Casting|CastToBP_Lobbymode (Game|GetGameMode)))
  (Utilities|FlowControl|DoOnce false
    (:Completed
      (Default|AddStartTile _asbp_lobbymode))))

(event OnComponentEndOverlap(GenerateTile)
  (params (OverlappedComponent :type Primitive%20Component%20Object%20Reference) (OtherActor :type Actor%20Object%20Reference) (OtherComp :type Primitive%20Component%20Object%20Reference) (OtherBodyIndex :type Integer))
  ;[1 1 1] 액터 파괴
  (Utilities|Casting|CastToBP_LoobyPlayer OtherActor)
  (Utilities|FlowControl|Delay 3.0)
  (Actor|DestroyActor))

(event EventBeginPlay
  (bind _floorpos (Variables|Default|GetFloorPos))
  (for _index (range 0 (Utilities|Array|LastIndex _floorpos))
    (bind _returnvalue (AddComponent|AddChildActorComponent false (Utilities|Array|Get(acopy) _floorpos _index)))
    (ChildActorComponent|SetChildActorClass _returnvalue "/Game/Blueprint/Actor/BP_Floor2.BP_Floor2_C")))

(fn ConstructionScript
  (CallFunction|SetFloorNum)
  (CallFunction|SetFloorPosition))