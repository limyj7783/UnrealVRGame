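; BP_Scoreboard is an actor that carries two sets of small dart platforms and stays a set distance ahead of the player along X.
; The construction script reads arrow component transforms into A and B lists, then spawns a matching dart platform child actor at each.
; Tick repositions the board at fixed Y and height, and clears the game mode's IsGeneratedDartPlatform flag once no dart platforms of either type exist.
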(event EventTick
  (params (DeltaSeconds :type Float%20%28single-precision%29))
  (Utilities|FlowControl|Sequence
    (:then_0
      (Transformation|SetWorldLocation (Variables|Default|GetDefaultSceneRoot) (Math|Vector|MakeVector (+ (.X (Math|Vector|BreakVector (Transformation|GetActorLocation (Game|GetPlayerCharacter 0)))) (Variables|Default|GetDistanceToPlayer)) 0.0 2.5e+02) false false))
    (:then_1
      (bind _outactors (Actor|GetAllActorsOfClass "/Game/Blueprint/Actor/BP_SmallDartAPlatform.BP_SmallDartAPlatform_C"))
      (bind _outactors_2 (Actor|GetAllActorsOfClass "/Game/Blueprint/Actor/BP_SmallDartBPlatform.BP_SmallDartBPlatform_C"))
      (if (== (+ (Utilities|Array|Length _outactors_2) (Utilities|Array|Length _outactors)) 0)
        (bind _asbp_main_gamemode (Utilities|Casting|CastToBP_MainGamemode (Game|GetGameMode)))
        (Variables|/Game/Blueprint/Gamemode/MainGame/BP_MainGamemode.BP_MainGamemode_C|SetIsGeneratedDartPlatform _asbp_main_gamemode false)))))

(fn ConstructionScript
  (CallFunction|SetDartPlatform)
  (CallFunction|GenerateDartPlatform))

(fn SetDartPlatform
  (Variables|Default|SetDartAPlatform (Utilities|Array|MakeArray (Transformation|GetRelativeTransform (Variables|Default|GetArrow)) (Transformation|GetRelativeTransform (Variables|Default|GetArrow2)) (Transformation|GetRelativeTransform (Variables|Default|GetArrow5)) (Transformation|GetRelativeTransform (Variables|Default|GetArrow7)) (Transformation|GetRelativeTransform (Variables|Default|GetArrow8)) (Transformation|GetRelativeTransform (Variables|Default|GetArrow10))))
  (Variables|Default|SetDartBPlatform (Utilities|Array|MakeArray (Transformation|GetRelativeTransform (Variables|Default|GetArrow1)) (Transformation|GetRelativeTransform (Variables|Default|GetArrow3)) (Transformation|GetRelativeTransform (Variables|Default|GetArrow4)) (Transformation|GetRelativeTransform (Variables|Default|GetArrow6)) (Transformation|GetRelativeTransform (Variables|Default|GetArrow9)) (Transformation|GetRelativeTransform (Variables|Default|GetArrow11)))))

(fn GenerateDartPlatform
  (bind _dartaplatform (Variables|Default|GetDartAPlatform))
  (bind _dartbplatform (Variables|Default|GetDartBPlatform))
  (Utilities|FlowControl|Sequence
    (:then_0
      (for _index (range 0 (Utilities|Array|LastIndex _dartaplatform))
        (bind _returnvalue (AddComponent|AddChildActorComponent false (Utilities|Array|Get(acopy) _dartaplatform _index)))
        (ChildActorComponent|SetChildActorClass _returnvalue "/Game/Blueprint/Actor/BP_SmallDartAPlatform.BP_SmallDartAPlatform_C")))
    (:then_1
      (for _index_2 (range 0 (Utilities|Array|LastIndex _dartbplatform))
        (bind _returnvalue_2 (AddComponent|AddChildActorComponent false (Utilities|Array|Get(acopy) _dartbplatform _index_2)))
        (ChildActorComponent|SetChildActorClass _returnvalue_2 "/Game/Blueprint/Actor/BP_SmallDartBPlatform.BP_SmallDartBPlatform_C")))))