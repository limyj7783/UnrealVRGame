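; BP_Aim is an aim indicator actor that mirrors the player's current aim material and removes itself when the player dies.
; On BeginPlay and again every Tick, it casts player character 0 to BP_MainGamePlayer and applies CurrentAimMaterial to the SMAim mesh.
; Tick then polls the player's IsDeath flag and destroys the actor once it is true.
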(event EventBeginPlay
  (bind _asbp_main_game_player (Utilities|Casting|CastToBP_MainGamePlayer (Game|GetPlayerCharacter 0)))
  (Rendering|Material|SetMaterial (Variables|Default|GetSM_Aim) 0 (Variables|/Game/Blueprint/Gamemode/MainGame/BP_MainGamePlayer.BP_MainGamePlayer_C|GetCurrentAimMaterial _asbp_main_game_player)))

(event EventTick
  (params (DeltaSeconds :type Float%20%28single-precision%29))
  (Utilities|FlowControl|Sequence
    (:then_0
      (bind _asbp_main_game_player (Utilities|Casting|CastToBP_MainGamePlayer (Game|GetPlayerCharacter 0)))
      (Rendering|Material|SetMaterial (Variables|Default|GetSM_Aim) 0 (Variables|/Game/Blueprint/Gamemode/MainGame/BP_MainGamePlayer.BP_MainGamePlayer_C|GetCurrentAimMaterial _asbp_main_game_player)))
    (:then_1
      (bind _asbp_main_game_player_2 (Utilities|Casting|CastToBP_MainGamePlayer (Game|GetPlayerCharacter 0)))
      (if (Variables|/Game/Blueprint/Gamemode/MainGame/BP_MainGamePlayer.BP_MainGamePlayer_C|GetIsDeath _asbp_main_game_player_2)
        (Actor|DestroyActor)))))

(fn ConstructionScript)