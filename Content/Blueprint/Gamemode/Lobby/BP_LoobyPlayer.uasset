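; Lobby player pawn that looks around via input axes, drifts along world +X on Tick, and clicks UI through WidgetInteraction with the right motion controller trigger or L key.
; SetSelectedWeapon turns Q/W/E into a flag array, which SetCurrentWeapon uses to copy that slot's weapon data from parallel arrays.
; Helpers to tint weapon widgets and award score per X distance travelled are defined but not called in this graph.
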(event EventTick
  (params (DeltaSeconds :type Float%20%28single-precision%29))
  ;[1 1 1] 이동
  (Utilities|FlowControl|Sequence
    (:then_0
      (Pawn|Input|AddMovementInput "1.000000, 0, 0" (* DeltaSeconds 1.5e+02) false))))

(event Input|AxisEvents|InputAxisLoopUP
  (params (AxisValue :type Float%20%28single-precision%29))
  ;[1 1 1] 카메라 회전
  (Pawn|Input|AddControllerPitchInput AxisValue))

(event Input|AxisEvents|InputAxisLoopRight
  (params (AxisValue :type Float%20%28single-precision%29))
  ;[1 1 1] 카메라 회전
  (Pawn|Input|AddControllerYawInput AxisValue))

(event Input|KeyboardEvents|MotionControllerRightTrigger
  (params (Key :type Key%20Structure :default "AnyKey"))
  (bind _widgetinteraction (Variables|Default|GetWidgetInteraction))
  (:Pressed
    (Class|WidgetInteractionComponent|PressPointerKey _widgetinteraction "LeftMouseButton"))
  (:Released
    (Class|WidgetInteractionComponent|ReleasePointerKey _widgetinteraction "LeftMouseButton")))

(event Input|KeyboardEvents|L
  (params (Key :type Key%20Structure :default "AnyKey"))
  (bind _widgetinteraction (Variables|Default|GetWidgetInteraction))
  (:Pressed
    (Class|WidgetInteractionComponent|PressPointerKey _widgetinteraction "LeftMouseButton"))
  (:Released
    (Class|WidgetInteractionComponent|ReleasePointerKey _widgetinteraction "LeftMouseButton")))

(fn ConstructionScript)

(fn SetSelectedWeapon
  (params (SelectedWeapon :type String))
  (if (Utilities|Enum|Equal(Enum) SelectedWeapon "Q")
    (LocalVariables|SetIsSelectedWeaponQ true)
    (LocalVariables|SetIsSelectedWeaponW false)
    (LocalVariables|SetIsSelectedWeaponE false :!label _label)
    (Variables|WeaponInfom|SetSelectedWeapon (Utilities|Array|MakeArray (LocalVariables|GetIsSelectedWeaponQ) (LocalVariables|GetIsSelectedWeaponW) (LocalVariables|GetIsSelectedWeaponE)) :!label _label_2)
    (CallFunction|SetCurrentWeapon)
    (else
      (LocalVariables|SetIsSelectedWeaponQ false)
      (if (Utilities|Enum|Equal(Enum) SelectedWeapon "W")
        (LocalVariables|SetIsSelectedWeaponW true)
        (goto _label)
        (else
          (LocalVariables|SetIsSelectedWeaponW false)
          (if (Utilities|Enum|Equal(Enum) SelectedWeapon "E")
            (LocalVariables|SetIsSelectedWeaponE true)
            (goto _label_2)))))))

(fn PaintWidget
  (for _index (range 0 (Utilities|Array|LastIndex (Variables|WeaponInfom|GetSelectedWeapon)))
    (if (Utilities|Array|Get(acopy) (Variables|WeaponInfom|GetSelectedWeapon) _index)
      (Appearance|SetColorandOpacity (Utilities|Array|Get(acopy) (Variables|Wedget|GetWeaponWidget) _index) "(R=1.000000,G=0.000000,B=0.000000,A=1.000000)" :!class /Script/UMG.Image)
      (else
        (Appearance|SetColorandOpacity (Utilities|Array|Get(acopy) (Variables|Wedget|GetWeaponWidget) _index) "(R=1.000000,G=1.000000,B=1.000000,A=1.000000)" :!class /Script/UMG.Image)))))

(fn SetCurrentWeapon
  (for _index (range 0 (Utilities|Array|LastIndex (Variables|WeaponInfom|GetSelectedWeapon)))
    (if (Utilities|Array|Get(acopy) (Variables|WeaponInfom|GetSelectedWeapon) _index)
      (bind _output_get (Variables|WeaponInfom|SetWeaponIndex _index))
      (Variables|CurrentWeapon|SetCurrentWeaponMesh (Utilities|Array|Get(acopy) (Variables|WeaponInfom|GetWeaponMesh) _output_get))
      (Variables|CurrentWeapon|SetCurrentAimTexture (Utilities|Array|Get(acopy) (Variables|WeaponInfom|GetWeaponAimTexture) (Variables|WeaponInfom|GetWeaponIndex)))
      (Variables|CurrentWeapon|SetCurrentBulletCount (Utilities|Array|Get(acopy) (Variables|WeaponInfom|GetWeaponBulletCount) (Variables|WeaponInfom|GetWeaponIndex)))
      (Variables|CurrentWeapon|SetCurrentBullet (Utilities|Array|Get(acopy) (Variables|WeaponInfom|GetWeaponBullet) (Variables|WeaponInfom|GetWeaponIndex)))
      (Variables|CurrentWeapon|SetCurrentCoolTime (Utilities|Array|Get(acopy) (Variables|WeaponInfom|GetWeaponCoolTime) (Variables|WeaponInfom|GetWeaponIndex)))
      (Variables|CurrentWeapon|SetCurrentTransform (Utilities|Array|Get(acopy) (Variables|WeaponInfom|GetWeaponTransform) (Variables|WeaponInfom|GetWeaponIndex)))
      (Variables|CurrentWeapon|SetCurrentFireSound (Utilities|Array|Get(acopy) (Variables|WeaponInfom|GetFireSound) (Variables|WeaponInfom|GetWeaponIndex)))
      (Variables|CurrentWeapon|SetCurrentArrowComponent (Utilities|Array|Get(acopy) (Variables|WeaponInfom|GetWeaponArrowComponentLcation) (Variables|WeaponInfom|GetWeaponIndex))))))

(fn IncreseScorebyLocationX
  (bind _output_get (Variables|LocationToScore|SetCurrentLocation.X (.X (Math|Vector|BreakVector (Transformation|GetActorLocation)))))
  (Variables|LocationToScore|SetDeltaLocation.X (+ (- _output_get (Variables|LocationToScore|GetLastLocation.X)) (Variables|LocationToScore|GetDeltaLocation.X)))
  (Variables|LocationToScore|SetLastLocation.X _output_get)
  (if (> (Variables|LocationToScore|GetDeltaLocation.X) 1e+03)
    (Variables|LocationToScore|SetDeltaLocation.X 0.0)
    (Variables|Player|SetCurrentScore (+ (Variables|Player|GetCurrentScore) 10))))