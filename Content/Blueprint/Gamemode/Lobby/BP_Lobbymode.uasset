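; Lobby game mode that builds a chained platform track and offers spawn helpers for items and UI actors.
; BeginPlay spawns five lobby platforms, each placed at the previous one's AttachPoint via NextAP; AddTile does the same with BP_PlatformParent.
; The construction script flags whether an HMD is connected.
; Other functions play an event sound, spawn item boxes ahead at random Y, and spawn or move UI actors, all relative to the player.
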(event EventBeginPlay
  ;[1 1 1] 기본 타일 생성
  (CallFunction|AddStartTile)
  (CallFunction|AddStartTile)
  (CallFunction|AddStartTile)
  (CallFunction|AddStartTile)
  (CallFunction|AddStartTile))

(fn ConstructionScript
  (bind _output_get (Variables|Default|SetHMDDeviceName (Class|HeadMountedDisplayFunctionLibrary|GetHMDDeviceName)))
  (if (Utilities|Name|Equal(Name) _output_get "None")
    (Variables|Default|SetIsConnectedHmd false)
    (else
      (Variables|Default|SetIsConnectedHmd true))))

(fn AddTile
  (bind _returnvalue (Game|SpawnActorfromClass "/Game/Blueprint/Actor/Parent/BP_PlatformParent.BP_PlatformParent_C" (Variables|Default|GetNextAP) "Undefined" 0 0))
  (Variables|Default|SetNextAP (Transformation|GetWorldTransform (Variables|/Game/Blueprint/Actor/Parent/BP_PlatformParent.BP_PlatformParent_C|GetAttachPoint _returnvalue))))

(fn AddStartTile
  (bind _returnvalue (Game|SpawnActorfromClass "/Game/Blueprint/Actor/BP_LobbyPlatform.BP_LobbyPlatform_C" (Variables|Default|GetNextAP) "Undefined" 0 0))
  (Variables|Default|SetNextAP (Transformation|GetWorldTransform (Variables|/Game/Blueprint/Actor/Parent/BP_PlatformParent.BP_PlatformParent_C|GetAttachPoint _returnvalue))))

(fn SoundPlay
  (Audio|PlaySoundatLocation "/Game/Sound/Cue/Cue_EventSound.Cue_EventSound" (Transformation|GetActorLocation (Game|GetPlayerCharacter 0))))

(fn GenerateItemBox
  (Game|SpawnActorfromClass "/Game/Blueprint/Actor/BP_ItemBox.BP_ItemBox_C" (Math|Transform|MakeTransform (Math|Vector|MakeVector (+ (.X (Math|Vector|BreakVector (Transformation|GetActorLocation (Game|GetPlayerCharacter 0)))) 3e+03) (Math|Random|RandomFloatinRange -2e+02 2e+02) 7e+01) "0, 0, 0" "1.000000,1.000000,1.000000") "Undefined" 0 0))

(fn SpawnUI
  (params (AddLocation :type Vector) (SpawnActor :type Actor%20Class%20Reference))
  (bind _returnvalue (Game|GetPlayerCharacter 0))
  (bind _returnvalue_2 (Transformation|GetActorTransform _returnvalue))
  (bind (_location _rotation _scale) (Math|Transform|BreakTransform _returnvalue_2))
  (bind _returnvalue_3 (Game|SpawnActorfromClass SpawnActor (Math|Transform|MakeTransform (+ _location AddLocation) "0,-180.000000, 0" _scale) "Undefined" 0 0))
  (return _returnvalue_3))

(fn MovementUI
  (params (AddLocation :type Vector) (UI :type Actor%20Object%20Reference))
  (Transformation|SetActorLocation UI (+ (Transformation|GetActorLocation (Game|GetPlayerCharacter 0)) AddLocation) false false))