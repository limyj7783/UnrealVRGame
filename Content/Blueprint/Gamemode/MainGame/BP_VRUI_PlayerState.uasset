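; VR UI actor, named for player state display, that repositions itself every tick to follow the first player character.
; It stays a fixed distance along world X from the player with constant height, rotation and scale.
; Its Y trails the player by an offset but is clamped to a lower limit, implemented as a branch between two transform updates.
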(event EventTick
  (params (DeltaSeconds :type Float%20%28single-precision%29))
  (bind _returnvalue (Game|GetPlayerCharacter 0))
  (bind _returnvalue_2 (Transformation|GetActorLocation _returnvalue))
  (bind (_x _y) (Math|Vector|BreakVector _returnvalue_2))
  (bind _returnvalue_3 (- _y 1e+02))
  (bind _returnvalue_4 (+ _x 1e+03))
  (if (< _returnvalue_3 -1.5e+02)
    (Transformation|SetActorTransform (Math|Transform|MakeTransform (Math|Vector|MakeVector _returnvalue_4 -1.5e+02 1e+02) "0,120.000000, 0"))
    (else
      (Transformation|SetActorTransform (Math|Transform|MakeTransform (Math|Vector|MakeVector _returnvalue_4 _returnvalue_3 1e+02) "0,120.000000, 0")))))

(fn ConstructionScript)