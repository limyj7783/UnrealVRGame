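; Player character for the main game, an auto-running shooter with VR input that moves forward until HP runs out, scoring by distance travelled.
; Keys or left thumbstick pick one of three weapons, loading mesh, bullet, ammo, cooldown and sound from parallel arrays.
; Attack spawns bullets along camera rotation, with cooldown starting on release.
; Each tick a line trace positions a separate BP_Aim actor, and a widget interaction component handles UI clicks.
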(event EventBeginPlay
  ;[1 1 1] 에임 큐브 생성
  (bind _returnvalue (Game|SpawnActorfromClass "/Game/Blueprint/Actor/BP_Aim.BP_Aim_C" (Math|Transform|MakeTransform "-1000.000000, 0, 0") "Undefined" 0 0))
  (Variables|Bullet|SetAimBP _returnvalue)
  ;[1 1 1] BulletCount 위젯 Visiblilty 세팅
  (bind _asbp_main_gamemode (Utilities|Casting|CastToBP_MainGamemode (Game|GetGameMode)))
  (if (Variables|/Game/Blueprint/Gamemode/MainGame/BP_MainGamemode.BP_MainGamemode_C|GetIsConnectedHMD _asbp_main_gamemode)
    _
    (else
      _))
  (Rendering|SetVisibility (Variables|Default|GetWidget_BulletCount) true false))

(event EventTick
  (params (DeltaSeconds :type Float%20%28single-precision%29))
  (bind _aimbp (Variables|Bullet|GetAimBP))
  (bind _arrow1 (Variables|Default|GetArrow1))
  (bind _gunoffset (Variables|Bullet|GetGunOffset))
  (bind _camera (Variables|Default|GetCamera))
  (bind _returnvalue (Transformation|GetWorldLocation _arrow1))
  (bind _returnvalue_2 (Transformation|GetWorldRotation _camera))
  (bind _returnvalue_3 (Math|Vector|RotateVector _gunoffset _returnvalue_2))
  (bind _returnvalue_4 (+ _returnvalue _returnvalue_3))
  ;[1 1 1] 생존
  (bind _isdeath (CallFunction|DeathJudgment))
  (bind _output_get (Variables|GameState|SetIsDeath _isdeath))
  (if (not _output_get)
    (Utilities|FlowControl|Sequence
      (:then_0
        (Pawn|Input|AddMovementInput "1.000000, 0, 0" (* DeltaSeconds 1.5e+02) false))
      (:then_1
        (CallFunction|IncreseScorebyLocationX))
      (:then_2
        ;;[1 1 1] 에임생성하는 라인 트레이스
        (bind _output_get_2 (Variables|Bullet|SetAimEndLocation (+ _returnvalue_4 (* (Math|Vector|GetForwardVector _camera) 1e+03))))
        (bind (_outhit _returnvalue_5) (Collision|LineTraceByChannel _returnvalue_4 _output_get_2 "TraceTypeQuery3" false 0 "None"))
        (if _returnvalue_5
          (Transformation|SetActorLocation _aimbp (.location _outhit) false false)
          (else
            (Transformation|SetActorLocation _aimbp (Variables|Bullet|GetAimEndLocation) false false)))))))

(event Input|ActionEvents|InputActionChoiceWeaponQ
  (params (Key :type Key%20Structure :default "AnyKey"))
  ;[1 1 1] 무기 선택
  (:Pressed
    (if (not (Variables|GameState|GetIsDeath))
      (CallFunction|SetSelectedWeapon "Q")
      (Components|StaticMesh|SetStaticMesh (Variables|Default|GetWeapon) (Variables|CurrentWeapon|GetCurrentWeaponMesh))
      (bind _asbp_main_gamemode (Utilities|Casting|CastToBP_MainGamemode (Game|GetGameMode)))
      (if (not (Variables|/Game/Blueprint/Gamemode/MainGame/BP_MainGamemode.BP_MainGamemode_C|GetIsConnectedHMD _asbp_main_gamemode))
        (CallFunction|PaintWidget)))))

(event Input|ActionEvents|InputActionGamePause
  (params (Key :type Key%20Structure :default "AnyKey"))
  ;[1 1 1] 게임 일시정지
  (:Released
    (if (Variables|GameState|GetIsPaused)
      (Game|SetGamePaused false)
      (Variables|GameState|SetIsPaused false)
      (else
        (Game|SetGamePaused true)
        (Variables|GameState|SetIsPaused true)))))

(event Input|ActionEvents|InputActionAttack
  (params (Key :type Key%20Structure :default "AnyKey"))
  (bind _isdeath (Variables|GameState|GetIsDeath))
  (bind _weaponbulletcount (Variables|WeaponInfom|GetWeaponBulletCount))
  (bind _weaponindex (Variables|WeaponInfom|GetWeaponIndex))
  (bind _camera (Variables|Default|GetCamera))
  (bind _returnvalue (Transformation|GetWorldRotation _camera))
  ;[1 1 1] 공격
  (:Pressed
    (if (not _isdeath)
      (if (> (Utilities|Array|Get(acopy) (Variables|WeaponInfom|GetWeaponBulletCount) (Variables|WeaponInfom|GetWeaponIndex)) 0)
        (if (Variables|CurrentWeapon|GetCanShoot)
          (Game|SpawnActorfromClass (Variables|CurrentWeapon|GetCurrentBullet) (Math|Transform|MakeTransform (+ (Transformation|GetWorldLocation (Variables|Default|GetArrow1)) (Math|Vector|RotateVector (Variables|Bullet|GetGunOffset) _returnvalue)) _returnvalue "1.000000,1.000000,1.000000") "Undefined" 0 0)
          (Audio|PlaySoundatLocation (Variables|CurrentWeapon|GetCurrentFireSound) (Transformation|GetSocketLocation (Variables|Default|GetWeapon) "None"))
          (Utilities|Array|SetArrayElem _weaponbulletcount _weaponindex (- (Utilities|Array|Get(acopy) _weaponbulletcount _weaponindex) 1))
          (Variables|CurrentWeapon|SetCanShoot false)
          (Variables|CurrentWeapon|SetCurrentBulletCount (- (Variables|CurrentWeapon|GetCurrentBulletCount) 1))))))
  (:Released
    (if (not _isdeath)
      (Utilities|FlowControl|Delay (Variables|CurrentWeapon|GetCurrentCoolTime))
      (Variables|CurrentWeapon|SetCanShoot true))))

(event Input|ActionEvents|InputActionJump
  (params (Key :type Key%20Structure :default "AnyKey"))
  (bind _isdeath (Variables|GameState|GetIsDeath))
  ;[1 1 1] 이동
  (:Pressed
    (if (not _isdeath)
      (Character|Jump)))
  (:Released
    (if (not _isdeath)
      (Character|StopJumping))))

(event Input|ActionEvents|InputActionChoiceWeaponE
  (params (Key :type Key%20Structure :default "AnyKey"))
  ;[1 1 1] 무기 선택
  (:Pressed
    (if (not (Variables|GameState|GetIsDeath))
      (CallFunction|SetSelectedWeapon "E")
      (Components|StaticMesh|SetStaticMesh (Variables|Default|GetWeapon) (Variables|CurrentWeapon|GetCurrentWeaponMesh))
      (bind _asbp_main_gamemode (Utilities|Casting|CastToBP_MainGamemode (Game|GetGameMode)))
      (if (not (Variables|/Game/Blueprint/Gamemode/MainGame/BP_MainGamemode.BP_MainGamemode_C|GetIsConnectedHMD _asbp_main_gamemode))
        (CallFunction|PaintWidget)))))

(event Input|ActionEvents|InputActionChoiceWeaponW
  (params (Key :type Key%20Structure :default "AnyKey"))
  ;[1 1 1] 무기 선택
  (:Pressed
    (if (not (Variables|GameState|GetIsDeath))
      (CallFunction|SetSelectedWeapon "W")
      (Components|StaticMesh|SetStaticMesh (Variables|Default|GetWeapon) (Variables|CurrentWeapon|GetCurrentWeaponMesh))
      (bind _asbp_main_gamemode (Utilities|Casting|CastToBP_MainGamemode (Game|GetGameMode)))
      (if (not (Variables|/Game/Blueprint/Gamemode/MainGame/BP_MainGamemode.BP_MainGamemode_C|GetIsConnectedHMD _asbp_main_gamemode))
        (CallFunction|PaintWidget)))))

(event Input|AxisEvents|InputAxisMoveRight
  (params (AxisValue :type Float%20%28single-precision%29))
  ;[1 1 1] 이동
  (if (Variables|GameState|GetIsDeath)
    (Rendering|SetVisibility (Variables|Default|GetWidget_BulletCount) false false)
    (else
      (Pawn|Input|AddMovementInput "0,1.000000, 0" AxisValue false))))

(event Input|AxisEvents|InputAxisLoopUP
  (params (AxisValue :type Float%20%28single-precision%29))
  ;[1 1 1] 카메라 회전
  (Pawn|Input|AddControllerPitchInput AxisValue))

(event Input|AxisEvents|InputAxisLoopRight
  (params (AxisValue :type Float%20%28single-precision%29))
  ;[1 1 1] 카메라 회전
  (Pawn|Input|AddControllerYawInput AxisValue))

(event Input|KeyboardEvents|MotionControllerLeftThumbstick
  (params (Key :type Key%20Structure :default "AnyKey"))
  (bind _isdeath (Variables|GameState|GetIsDeath))
  ;[1 1 1] 모션 컨트롤러 키세팅
  (:Pressed
    (bind _output_get (Variables|VRCtrl|SetL_Thumbstick_X (Class|Actor|GetInputAxisKeyValue)))
    (bind _output_get_2 (Variables|VRCtrl|SetL_Thumbstick_Y (Class|Actor|GetInputAxisKeyValue)))
    (if (and (> _output_get 0.0) (< _output_get_2 (/ (Math|Trig|GetPI) 6.0)))
      ;[1 1 1] 무기 선택
      (if (not _isdeath)
        (CallFunction|SetSelectedWeapon "E")
        (Components|StaticMesh|SetStaticMesh (Variables|Default|GetWeapon) (Variables|CurrentWeapon|GetCurrentWeaponMesh) :!label _label)
        (bind _asbp_main_gamemode (Utilities|Casting|CastToBP_MainGamemode (Game|GetGameMode)))
        (if (not (Variables|/Game/Blueprint/Gamemode/MainGame/BP_MainGamemode.BP_MainGamemode_C|GetIsConnectedHMD _asbp_main_gamemode))
          (CallFunction|PaintWidget)))
      (elif (and (< (Variables|VRCtrl|GetL_Thumbstick_X) 0.0) (< (Variables|VRCtrl|GetL_Thumbstick_Y) (/ (Math|Trig|GetPI) 6.0)))
        (if (not _isdeath)
          (CallFunction|SetSelectedWeapon "Q")
          (goto _label))
        (elif (not _isdeath)
          (CallFunction|SetSelectedWeapon "W")
          (goto _label))))))

(event Input|KeyboardEvents|MotionControllerRightTrigger
  (params (Key :type Key%20Structure :default "AnyKey"))
  (bind _widgetinteraction (Variables|Default|GetWidgetInteraction))
  (:Pressed
    (Class|WidgetInteractionComponent|PressPointerKey _widgetinteraction "LeftMouseButton"))
  (:Released
    (Class|WidgetInteractionComponent|ReleasePointerKey _widgetinteraction "LeftMouseButton")))

(event Input|KeyboardEvents|L
  (params (Key :type Key%20Structure :default "AnyKey"))
  (bind _widgetinteraction (Variables|Default|GetWidgetInteraction))
  (:Pressed
    (Class|WidgetInteractionComponent|PressPointerKey _widgetinteraction "LeftMouseButton"))
  (:Released
    (Class|WidgetInteractionComponent|ReleasePointerKey _widgetinteraction "LeftMouseButton")))

(fn ConstructionScript
  (CallFunction|SetSelectedWeapon "Q")
  (Variables|LocationToScore|SetCurrentLocation.X (.X (Math|Vector|BreakVector (Transformation|GetActorLocation))))
  (bind _asbp_main_gamemode (Utilities|Casting|CastToBP_MainGamemode (Game|GetGameMode)))
  (Variables|GameState|SetHMDDeviceName (Variables|/Game/Blueprint/Gamemode/MainGame/BP_MainGamemode.BP_MainGamemode_C|GetHMDDeviceName _asbp_main_gamemode)))

(fn SetSelectedWeapon
  (params (SelectedWeapon :type String))
  (if (Utilities|Enum|Equal(Enum) SelectedWeapon "Q")
    (LocalVariables|SetIsSelectedWeaponQ true)
    (LocalVariables|SetIsSelectedWeaponW false)
    (LocalVariables|SetIsSelectedWeaponE false :!label _label)
    (Variables|WeaponInfom|SetSelectedWeapon (Utilities|Array|MakeArray (LocalVariables|GetIsSelectedWeaponQ) (LocalVariables|GetIsSelectedWeaponW) (LocalVariables|GetIsSelectedWeaponE)) :!label _label_2)
    (CallFunction|SetCurrentWeapon)
    (else
      (LocalVariables|SetIsSelectedWeaponQ false)
      (if (Utilities|Enum|Equal(Enum) SelectedWeapon "W")
        (LocalVariables|SetIsSelectedWeaponW true)
        (goto _label)
        (else
          (LocalVariables|SetIsSelectedWeaponW false)
          (if (Utilities|Enum|Equal(Enum) SelectedWeapon "E")
            (LocalVariables|SetIsSelectedWeaponE true)
            (goto _label_2)))))))

(fn PaintWidget
  (for _index (range 0 (Utilities|Array|LastIndex (Variables|WeaponInfom|GetSelectedWeapon)))
    (if (Utilities|Array|Get(acopy) (Variables|WeaponInfom|GetSelectedWeapon) _index)
      (Appearance|SetColorandOpacity (Utilities|Array|Get(acopy) (Variables|Wedget|GetWeaponWidget) _index) "(R=1.000000,G=0.000000,B=0.000000,A=1.000000)" :!class /Script/UMG.Image)
      (else
        (Appearance|SetColorandOpacity (Utilities|Array|Get(acopy) (Variables|Wedget|GetWeaponWidget) _index) "(R=1.000000,G=1.000000,B=1.000000,A=1.000000)" :!class /Script/UMG.Image)))))

(fn SetCurrentWeapon
  (for _index (range 0 (Utilities|Array|LastIndex (Variables|WeaponInfom|GetSelectedWeapon)))
    (if (Utilities|Array|Get(acopy) (Variables|WeaponInfom|GetSelectedWeapon) _index)
      (bind _output_get (Variables|WeaponInfom|SetWeaponIndex _index))
      (Variables|CurrentWeapon|SetCurrentWeaponMesh (Utilities|Array|Get(acopy) (Variables|WeaponInfom|GetWeaponMesh) _output_get))
      (Variables|CurrentWeapon|SetCurrentAimMaterial (Utilities|Array|Get(acopy) (Variables|WeaponInfom|GetWeaponAimMaterial) (Variables|WeaponInfom|GetWeaponIndex)))
      (Variables|CurrentWeapon|SetCurrentBulletCount (Utilities|Array|Get(acopy) (Variables|WeaponInfom|GetWeaponBulletCount) (Variables|WeaponInfom|GetWeaponIndex)))
      (Variables|CurrentWeapon|SetCurrentBullet (Utilities|Array|Get(acopy) (Variables|WeaponInfom|GetWeaponBullet) (Variables|WeaponInfom|GetWeaponIndex)))
      (Variables|CurrentWeapon|SetCurrentCoolTime (Utilities|Array|Get(acopy) (Variables|WeaponInfom|GetWeaponCoolTime) (Variables|WeaponInfom|GetWeaponIndex)))
      (Variables|CurrentWeapon|SetCurrentTransform (Utilities|Array|Get(acopy) (Variables|WeaponInfom|GetWeaponTransform) (Variables|WeaponInfom|GetWeaponIndex)))
      (Variables|CurrentWeapon|SetCurrentFireSound (Utilities|Array|Get(acopy) (Variables|WeaponInfom|GetFireSound) (Variables|WeaponInfom|GetWeaponIndex)))
      (bind _output_get_2 (Variables|CurrentWeapon|SetCurrentArrowComponent (Utilities|Array|Get(acopy) (Variables|WeaponInfom|GetWeaponArrowComponentLcation) (Variables|WeaponInfom|GetWeaponIndex))))
      (Transformation|SetRelativeLocation (Variables|Default|GetArrow1) _output_get_2 false false))))

(fn IncreseScorebyLocationX
  (bind _output_get (Variables|LocationToScore|SetCurrentLocation.X (.X (Math|Vector|BreakVector (Transformation|GetActorLocation)))))
  (Variables|LocationToScore|SetDeltaLocation.X (+ (- _output_get (Variables|LocationToScore|GetLastLocation.X)) (Variables|LocationToScore|GetDeltaLocation.X)))
  (Variables|LocationToScore|SetLastLocation.X _output_get)
  (if (> (Variables|LocationToScore|GetDeltaLocation.X) 1e+03)
    (Variables|LocationToScore|SetDeltaLocation.X 0.0)
    (Variables|Player|SetCurrentScore (+ (Variables|Player|GetCurrentScore) 10))))

(fn DeathJudgment
  (if (<= (Variables|Player|GetCurrentHP) 0.0)
    (return true)
    (else
      (return false))))