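; Main game mode that builds the opening platform track, starts background music and triggers random gameplay events.
; On BeginPlay it chains a start tile and two platform tiles, each spawned at the previous tile's AttachPoint via NextAP.
; Delays in Tick pace a probability roll for an event sound or item box ahead of the player, plus a one-time scoreboard spawn.
; The construction script records whether an HMD is connected.
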(event EventBeginPlay
  ;[1 1 1] 기본 타일 생성
  (CallFunction|AddStartTile)
  (CallFunction|AddTile)
  (CallFunction|AddTile)
  ;[1 1 1] 배경음
  (Audio|PlaySound2D "/Game/Sound/Cue/Cue_BGM.Cue_BGM"))

(event EventTick
  (params (DeltaSeconds :type Float%20%28single-precision%29))
  ;[1 1 1] 이벤트 사운드 재생 및 아이템 박스 생성
  (Utilities|FlowControl|Sequence
    (:then_0
      (Utilities|FlowControl|Delay 1.0)
      (if (> (Variables|Default|GetEventPercent) (Math|Random|RandomFloatinRange 0.0 1.0))
        (if (Math|Random|RandomBool)
          (CallFunction|SoundPlay)
          (else
            (CallFunction|GenerateItemBox)))))
    (:then_1
      ;[1 1 1] 스코어 보드 생성
      (if (not (Variables|Default|GetIsGeneratedDartPlatform))
        (Utilities|FlowControl|Delay 5.0)
        (Game|SpawnActorfromClass "/Game/Blueprint/Actor/BP_Scoreboard.BP_Scoreboard_C" (Math|Transform|MakeTransform "-500.000000, 0,250.000000") "Undefined" 0 0)
        (Variables|Default|SetIsGeneratedDartPlatform true)))))

(fn ConstructionScript
  (bind _output_get (Variables|Default|SetHMDDeviceName (Class|HeadMountedDisplayFunctionLibrary|GetHMDDeviceName)))
  (if (Utilities|Name|Equal(Name) _output_get "None")
    (Variables|Default|SetIsConnectedHMD false)
    (else
      (Variables|Default|SetIsConnectedHMD true))))

(fn AddTile
  (bind _returnvalue (Game|SpawnActorfromClass "/Game/Blueprint/Actor/Parent/BP_PlatformParent.BP_PlatformParent_C" (Variables|Default|GetNextAP) "Undefined" 0 0))
  (Variables|Default|SetNextAP (Transformation|GetWorldTransform (Variables|/Game/Blueprint/Actor/Parent/BP_PlatformParent.BP_PlatformParent_C|GetAttachPoint _returnvalue))))

(fn AddStartTile
  (bind _returnvalue (Game|SpawnActorfromClass "/Game/Blueprint/Actor/BP_Platform_Start.BP_Platform_Start_C" (Variables|Default|GetNextAP) "Undefined" 0 0))
  (Variables|Default|SetNextAP (Transformation|GetWorldTransform (Variables|/Game/Blueprint/Actor/Parent/BP_PlatformParent.BP_PlatformParent_C|GetAttachPoint _returnvalue))))

(fn SoundPlay
  (Audio|PlaySoundatLocation "/Game/Sound/Cue/Cue_EventSound.Cue_EventSound" (Transformation|GetActorLocation (Game|GetPlayerCharacter 0))))

(fn GenerateItemBox
  (Game|SpawnActorfromClass "/Game/Blueprint/Actor/BP_ItemBox.BP_ItemBox_C" (Math|Transform|MakeTransform (Math|Vector|MakeVector (+ (.X (Math|Vector|BreakVector (Transformation|GetActorLocation (Game|GetPlayerCharacter 0)))) 3e+03) (Math|Random|RandomFloatinRange -2e+02 2e+02) 7e+01) "0, 0, 0" "1.000000,1.000000,1.000000") "Undefined" 0 0))